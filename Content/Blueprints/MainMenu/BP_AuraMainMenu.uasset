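; Main menu setup Blueprint that starts the game's front-end on BeginPlay.
; It plays the menu music as a 2D sound and keeps a reference to it, then creates WBP_MainMenu and adds it to the viewport.
; Input switches to UI only with the menu focused and the mouse cursor shown.
; The UpdateTime and SinOfTime functions are inert stubs that the startup flow does not call.
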(event `self.ReceiveBeginPlay`
  (bind _returnvalue (`GameplayStatics.GetPlayerController` 0))
  (bind _returnvalue_2 (`GameplayStatics.SpawnSound2D` "/Game/Assets/Sounds/Music/Music_MainMenu.Music_MainMenu" 1.0 1.0 0.0 null))
  (set `self.MainMenuMusic` _returnvalue_2)
  (bind _returnvalue_3 (`|CreateWidget` "/Game/Blueprints/UI/MainMenu/WBP_MainMenu.WBP_MainMenu_C"))
  (`UserWidget.AddToViewport` _returnvalue_3 0)
  (`WidgetBlueprintLibrary.SetInputMode_UIOnlyEx` _returnvalue _returnvalue_3)
  (set `PlayerController.bShowMouseCursor` true _returnvalue))

(fn `SinOfTime`
  (returns (ReturnValue :type "Float (double-precision)"))
  (return (* (`KismetMathLibrary.Sin` 0.0) 0.0)))

(fn `UpdateTime`
  (params (A :type "Float (double-precision)")))

(fn `UserConstructionScript`)